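; BP_AppSink is an actor that shows video from a GStreamer pipeline on its Display component.
; The construction script passes the pipeline name, config and autostart setting to the GstPipeline component, and the same name to GstAppSink.
; When GstAppSink creates a texture, the actor builds a dynamic instance of VideoMaterial, feeds the texture into its Frame parameter and applies it to Display.
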(event OnGstTextureCreated(GstAppSink)
  (params (AppSink :type Gst%20App%20Sink%20Component%20Object%20Reference) (NewTexture :type Texture%202D%20Object%20Reference) (Format :type EGstVideoFormat%20Enum :default "GST_VIDEO_FORMAT_UNKNOWN") (Width :type Integer) (Height :type Integer))
  (bind _returnvalue (Rendering|Material|CreateDynamicMaterialInstance (Variables|GStreamer|GetVideoMaterial) "None" "None" :!class /Script/Engine.KismetMaterialLibrary))
  (Rendering|Material|SetTextureParameterValue _returnvalue "Frame" NewTexture)
  (Rendering|Material|SetMaterial (Variables|Default|GetDisplay) 0 _returnvalue))

(event EventBeginPlay)

(event EventTick
  (params (DeltaSeconds :type Float%20%28single-precision%29)))

(fn ConstructionScript
  (bind _gstpipeline (Variables|Default|GetGstPipeline))
  (Variables|/Script/GStreamer.GstPipelineComponent|SetPipelineName _gstpipeline (Variables|GStreamer|GetPipelineName))
  (Variables|/Script/GStreamer.GstPipelineComponent|SetPipelineConfig _gstpipeline (Variables|GStreamer|GetPipelineConfig))
  (Variables|/Script/GStreamer.GstPipelineComponent|SetPipelineAutostart _gstpipeline (Variables|GStreamer|GetAutostart))
  (Variables|/Script/GStreamer.GstAppSinkComponent|SetPipelineName (Variables|Default|GetGstAppSink) (Variables|GStreamer|GetPipelineName)))